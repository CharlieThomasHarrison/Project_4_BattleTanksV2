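; Player-controllable tank Blueprint that handles driving, aiming and firing input.
; BeginPlay registers the barrel and turret references and initialises TankMovement with the left and right tracks.
; Input either throttles each track directly or sends move and turn intents through TankMovement, while aim axes rotate the azimuth gimbal and spring arm, and Fire calls Fire().
; The construction script assigns both tracks' mesh and physical material.
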(event EventBeginPlay
  (Class|Tank|SetBarrelReference (Variables|Default|GetBarrel))
  (Class|Tank|SetTurretReference (Variables|Default|GetTurret))
  (Class|TankMovementComponent|Initialise (Variables|Default|GetTankMovement) (Variables|Default|GetLeft_Tank_Track) (Variables|Default|GetRight_Tank_Track)))

(event Input|ActionEvents|InputActionFire
  (params (Key :type Key%20Structure))
  ;[1 1 1] Aim Input Bindings
  (:Pressed
    (Class|Tank|Fire)))

(event Input|AxisEvents|InputAxisAimAzimuth
  (params (AxisValue :type Float%20%28single-precision%29))
  ;[1 1 1] Aim Input Bindings
  (Transformation|AddLocalRotation (Variables|Default|GetAzimuth%20Gimbal) (Math|Rotator|MakeRotator 0.0 0.0 AxisValue) false false))

(event Input|AxisEvents|InputAxisAimElevation
  (params (AxisValue :type Float%20%28single-precision%29))
  ;[1 1 1] Aim Input Bindings
  (Transformation|AddLocalRotation (Variables|Default|GetSpringArm) (Math|Rotator|MakeRotator 0.0 AxisValue 0.0) false false))

(event Input|AxisEvents|InputAxisLeftTrackThrottle
  (params (AxisValue :type Float%20%28single-precision%29))
  ;[1 1 1] Movement Input Bindings
  (Class|TankTrack|SetThrottle (Variables|Default|GetLeft_Tank_Track) AxisValue))

(event Input|AxisEvents|InputAxisRightTrackThrottle
  (params (AxisValue :type Float%20%28single-precision%29))
  ;[1 1 1] Movement Input Bindings
  (Class|TankTrack|SetThrottle (Variables|Default|GetRight_Tank_Track) AxisValue))

(event Input|AxisEvents|InputAxisMoveForward
  (params (AxisValue :type Float%20%28single-precision%29))
  ;[1 1 1] Movement Input Bindings
  (Class|TankMovementComponent|IntendMoveForward (Variables|Default|GetTankMovement) AxisValue))

(event Input|AxisEvents|InputAxisMoveBackward
  (params (AxisValue :type Float%20%28single-precision%29))
  ;[1 1 1] Movement Input Bindings
  (Class|TankMovementComponent|IntendMoveForward (Variables|Default|GetTankMovement) AxisValue))

(event Input|AxisEvents|InputAxisMoveRight
  (params (AxisValue :type Float%20%28single-precision%29))
  ;[1 1 1] Movement Input Bindings
  (Class|TankMovementComponent|IntendTurnRight (Variables|Default|GetTankMovement) AxisValue))

(event Input|AxisEvents|InputAxisMoveLeft
  (params (AxisValue :type Float%20%28single-precision%29))
  ;[1 1 1] Movement Input Bindings
  (Class|TankMovementComponent|IntendTurnLeft (Variables|Default|GetTankMovement) AxisValue))

(fn ConstructionScript
  (bind _left_tank_track (Variables|Default|GetLeft_Tank_Track))
  (bind _right_tank_track (Variables|Default|GetRight_Tank_Track))
  (Components|StaticMesh|SetStaticMesh _right_tank_track "/Game/models/tank_fbx_Track.tank_fbx_Track")
  (Class|PrimitiveComponent|SetPhysMaterialOverride _right_tank_track "/Game/Material/Track.Track")
  (Components|StaticMesh|SetStaticMesh _left_tank_track "/Game/models/tank_fbx_Track.tank_fbx_Track")
  (Class|PrimitiveComponent|SetPhysMaterialOverride _left_tank_track "/Game/Material/Track.Track"))